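; State Tree task that makes a TBPlayer AI stop the ball with a motion-warped animation.
; On entering the state it flags the animation component as stopping, moves toward the ball and turns to face it horizontally.
; It sets a warp target at the ball's position projected ahead by its physics velocity, then plays the stop-ball montage.
; After the montage's duration it clears the flag and finishes successfully.
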(event EventLatentEnterState
  (params (Transition :type State%20Tree%20Transition%20Result%20Structure%20%28by%20ref%29))
  (bind _returnvalue (Actor|GetActorOfClass "/Game/Ball/BP_Ball1.BP_Ball1_C"))
  (bind _astbplayer (Utilities|Casting|CastToTBPlayer (Variables|Context|GetActor)))
  (Class|TBPlayerAnimationComponent|SetStoppingBall (Actor|GetComponentbyClass _astbplayer "/Script/TestBall.TBPlayerAnimationComponent") true)
  (Class|TBPlayer|MovetoLocation _astbplayer (Transformation|GetActorLocation _returnvalue))
  (bind _returnvalue_2 (Class|Ball1|GetBallPhysicVelocity _returnvalue))
  (Transformation|SetActorRotation _astbplayer (Math|Conversions|RotationFromXVector (* (- (Transformation|GetActorLocation _returnvalue) (Transformation|GetActorLocation _astbplayer)) "1.000000,1.000000,0.000000")))
  (Class|MotionWarpingComponent|AddorUpdateWarpTargetfromTransform (Actor|GetComponentbyClass _astbplayer "/Script/MotionWarping.MotionWarpingComponent") "StopBallWarp" (Math|Transform|MakeTransform (+ (* _returnvalue_2 0.35) (Transformation|GetActorLocation _returnvalue)) (Math|Conversions|RotationFromXVector (* (- (Transformation|GetActorLocation _returnvalue) (Transformation|GetActorLocation _astbplayer)) "1.000000,1.000000,0.000000"))))
  (bind _returnvalue_3 (Animation|PlayAnimMontage _astbplayer "/Game/Animation/Animation/Montages/AM_StopBallModified.AM_StopBallModified" 1.0 "None"))
  (Utilities|FlowControl|Delay _returnvalue_3)
  (Class|TBPlayerAnimationComponent|SetStoppingBall (Actor|GetComponentbyClass _astbplayer "/Script/TestBall.TBPlayerAnimationComponent") false)
  (StateTree|FinishTask true))